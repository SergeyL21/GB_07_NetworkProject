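; Multiplayer game mode that sorts joining player controllers into two balanced teams.
; On post login it puts the player in Team B only when Team A is larger, otherwise Team A, and sets the team ID.
; It then names the player from the team and slot index through a server call.
; On logout it removes the controller from its team array.
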(event `self.K2_PostLogin`
  (params (NewPlayer :type "PlayerController Object Reference"))
  ;[1 1 1] Event On Post Login
  (bind _asbp_multiplayer_player_controller (cast `/Game/Blueprints/BP_MultiplayerPlayerController` NewPlayer)
    (:`then`
      (if (> (`KismetArrayLibrary.Array_Length` (`self.TeamA`)) (`KismetArrayLibrary.Array_Length` (`self.TeamB`)))
        (`/Game/Blueprints/BP_MultiplayerPlayerController.SetTeamID` _asbp_multiplayer_player_controller 2)
        (bind _returnvalue (`KismetArrayLibrary.Array_Add` (`self.TeamB`) _asbp_multiplayer_player_controller))
        (set `self.CurrentPlayerIndex` _returnvalue)
        (else
          (`/Game/Blueprints/BP_MultiplayerPlayerController.SetTeamID` _asbp_multiplayer_player_controller 1)
          (bind _returnvalue_2 (`KismetArrayLibrary.Array_Add` (`self.TeamA`) _asbp_multiplayer_player_controller))
          (set `self.CurrentPlayerIndex` _returnvalue_2)))
      (`/Game/Blueprints/BP_MultiplayerPlayerController.Server_SetPlayerName` _asbp_multiplayer_player_controller (`KismetTextLibrary.Conv_TextToString` (`|FormatText` "Team{1}_Player{2}" (`/Game/Blueprints/BP_MultiplayerPlayerController.TeamID` _asbp_multiplayer_player_controller) (+ (`self.CurrentPlayerIndex`) 1)))))
    (:`CastFailed`
      (`KismetSystemLibrary.PrintString` "Post login player controller error!" true true (struct :`R` 1.0 :`A` 1.0)))))

(event `self.K2_OnLogout`
  (params (ExitingController :type "Controller Object Reference"))
  (bind _teama (`self.TeamA`))
  (bind _teamb (`self.TeamB`))
  ;[1 1 1] Event On Logout
  (bind _asbp_multiplayer_player_controller (cast `/Game/Blueprints/BP_MultiplayerPlayerController` ExitingController))
  (switch `int` (`KismetMathLibrary.Conv_ByteToInt` (`/Game/Blueprints/BP_MultiplayerPlayerController.TeamID` _asbp_multiplayer_player_controller))
    (:`1`
      (`KismetArrayLibrary.Array_Remove` _teama (`KismetArrayLibrary.Array_Find` _teama _asbp_multiplayer_player_controller)))
    (:`2`
      (`KismetArrayLibrary.Array_Remove` _teamb (`KismetArrayLibrary.Array_Find` _teamb _asbp_multiplayer_player_controller)))))

(fn `UserConstructionScript`)