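; Multiplayer projectile that flies forward, damages characters and destroys itself on impact or when its lifetime timer expires.
; The server moves it every tick by setting location without sweep and handles sphere overlaps, ignoring the owner.
; Hitting a BP_MultiplayerCharacter applies damage through its health component.
; That hit, or one on another projectile, multicasts an explosion, disables overlaps and destroys the projectile after a short delay.
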(event `self.ReceiveBeginPlay`
  ;[1 1 1] Event Begin Section
  (`KismetSystemLibrary.K2_SetTimerDelegate` (delegate `Client Lifetime Ended`) (`self.Lifetime`)))

(event `self.ReceiveTick`
  (params (DeltaSeconds :type "Float (single-precision)"))
  ;[1 1 1] Event Tick Section
  (if (`KismetSystemLibrary.IsServer`)
    (`self.Server Move` DeltaSeconds)))

(event `Client Lifetime Ended`
  ;[1 1 1] Event Begin Section
  (`self.Server Lifetime Ended`))

(event `Server Lifetime Ended`
  ;[0.06667 0.6039 1] Server Lifetime Ended
  (`KismetSystemLibrary.Delay` 0.2)
  (`self.K2_DestroyActor`))

(event `Server Move`
  (params (`Delta Time` :type "Float (double-precision)"))
  ;[1 1 1] Projectile Movement
  (`self.K2_SetActorLocation` (+ (`self.K2_GetActorLocation`) (* (`self.GetActorForwardVector`) (* `Delta Time` (`self.Speed`))))))

(event `self.Sphere Collision.OnComponentBeginOverlap`
  (params (OverlappedComponent :type "PrimitiveComponent Object Reference") (OtherActor :type "Actor Object Reference") (OtherComp :type "PrimitiveComponent Object Reference") (OtherBodyIndex :type Integer) (bFromSweep :type Boolean) (SweepResult :type "HitResult Structure (by ref)"))
  ;[1 1 1] On Component Begin Overlap
  (if (`KismetSystemLibrary.IsServer`)
    (`self.Server Collision` OtherActor (`self.K2_GetActorLocation`))))

(event `Server Collision`
  (params (`Other Actor` :type "Actor Object Reference") (Location :type "Vector Structure"))
  ;[0.06667 0.6039 1] Server Collision
  (if (!= `Other Actor` (`self.GetOwner`))
    (bind _asbp_multiplayer_character (cast `/Game/Blueprints/BP_MultiplayerCharacter` `Other Actor`)
      (:`then`
        (`/Game/Blueprints/BP_HealthComponent.Take Damage` (`/Game/Blueprints/BP_MultiplayerCharacter.BP_HealthComponent` _asbp_multiplayer_character) (`self.Damage`)))
      (:`CastFailed`
        (cast `/Game/Blueprints/BP_Projectile` `Other Actor`)))
    (`self.Multicast Hit Effect` Location)
    (set `PrimitiveComponent.bGenerateOverlapEvents` false (`self.Sphere Collision`))
    (`self.Server Lifetime Ended`)))

(event `Spawn Hit Effect`
  (params (`Hit Location` :type "Vector Structure"))
  ;[1 1 1] Spawn Hit Effect
  (`GameplayStatics.SpawnEmitterAtLocation` "/Game/Particles/P_Explosion.P_Explosion" `Hit Location`))

(event `Multicast Hit Effect`
  (params (`Hit Location` :type "Vector Structure"))
  ;[1 1 1] Multicast Hit Effect
  (`self.Spawn Hit Effect ` `Hit Location`))

(fn `UserConstructionScript`)