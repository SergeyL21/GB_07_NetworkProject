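; Game instance that manages LAN multiplayer sessions: hosting, searching and joining.
; CreateGame creates a session and, on success, opens Level_01 as a listen server.
; FindGames caches search results in Sessions and calls OnSessionFindingFinished; GetGames exposes that list, and JoinToGame joins an entry by validated index.
; Session failures and network errors are only reported as red on-screen prints.
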(event `Create Game`
  ;[1 1 1] Create Session
  (`CreateSessionCallbackProxy.CreateSession` (`GameplayStatics.GetPlayerController` 0) 16 true
    (:`OnSuccess`
      (`GameplayStatics.OpenLevel` "Level_01" true "listen"))
    (:`OnFailure`
      (`KismetSystemLibrary.PrintString` "Game creation error!" true true (struct :`R` 1.0 :`A` 1.0) 5.0))))

(event `Find Games`
  ;[1 1 1] Find Games
  (bind _results (`FindSessionsCallbackProxy.FindSessions` (`GameplayStatics.GetPlayerController` 0) 20 true)
    (:`OnSuccess`
      (set `self.Sessions` _results)
      (`self.OnSessionFindingFinished`))
    (:`OnFailure`
      (`KismetSystemLibrary.PrintString` "Game searching error!" true true (struct :`R` 1.0 :`A` 1.0) 5.0))))

(event `Join To Game`
  (params (`Session Index` :type Integer))
  (bind _sessions (`self.Sessions`))
  ;[1 1 1] Join To Game
  (if (`KismetArrayLibrary.Array_IsValidIndex` _sessions `Session Index`)
    (`JoinSessionCallbackProxy.JoinSession` (`GameplayStatics.GetPlayerController` 0) (`|GetArrayItem` _sessions `Session Index`)
      (:`OnFailure`
        (`KismetSystemLibrary.PrintString` "Join to game error!" true true (struct :`R` 1.0 :`A` 1.0))))))

(event `self.HandleNetworkError`
  (params (FailureType :type "ENetworkFailure Enum" :default "NetDriverAlreadyExists") (bIsServer :type Boolean))
  ;[1 1 1] Network errors handle
  (`KismetSystemLibrary.PrintString` (`KismetStringLibrary.Concat_StrStr` "Network error: " (`|GetEnumeratorNameAsString` FailureType) "(is server =" (`KismetStringLibrary.Conv_BoolToString` bIsServer) ")") true true (struct :`R` 1.0 :`A` 1.0) 5.0))

(fn `Get Games`
  (returns (Sessions :type "Array of BlueprintSessionResult Structure"))
  (return (`self.Sessions`)))