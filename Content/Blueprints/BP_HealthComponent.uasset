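; Health component that tracks current and max health for a multiplayer character.
; TakeDamage forwards to ServerTakeDamage, which subtracts the damage from CurrentHealth without clamping or a death check.
; The CurrentHealth RepNotify prints a debug message and tells the owning BP_MultiplayerCharacter to update its health bar widget.
; The MaxHealth RepNotify is empty.
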(event `Take Damage`
  (params (`Damage Value` :type "Float (double-precision)"))
  (`self.Server Take Damage` `Damage Value`))

(event `Server Take Damage`
  (params (`Damage Value` :type "Float (double-precision)"))
  (set `self.Current Health` (- (`self.Current Health`) `Damage Value`)))

(fn `OnRep_Current Health`
  (`KismetSystemLibrary.PrintString` (`KismetTextLibrary.Conv_TextToString` (`|FormatText` "HEALTH: {0}/{1}" (`self.Current Health`) (`self.Max Health`))) true true (struct :`R` 1.0 :`B` 0.039589 :`A` 1.0) 3.0)
  (bind _asbp_multiplayer_character (cast `/Game/Blueprints/BP_MultiplayerCharacter` (`self.GetOwner`)))
  (`/Game/Blueprints/BP_MultiplayerCharacter.Update Health Bar Widget` _asbp_multiplayer_character (`self.Current Health`) (`self.Max Health`)))

(fn `OnRep_Max Health`)